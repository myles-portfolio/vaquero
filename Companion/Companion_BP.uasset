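; Companion NPC character that takes follow, stay, go-to and talk commands from the game.
; Commands set targets and states on its CompanionController_BP, which receives the DialogueTree on BeginPlay.
; Talking also plays a salute montage and removes the interaction prompt.
; Sphere overlaps register the NPC with PlayerAvatar_BP and manage a screen-space "Talk" widget, created behind a DoOnce with no reset.
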(event OnComponentBeginOverlap(Sphere)
  (params (OverlappedComponent :type Primitive%20Component%20Object%20Reference) (OtherActor :type Actor%20Object%20Reference) (OtherComp :type Primitive%20Component%20Object%20Reference) (OtherBodyIndex :type Integer) (bFromSweep :type Boolean) (SweepResult :type Hit%20Result%20Structure%20%28by%20ref%29))
  ;[1 1 1] Interaction Text Show/Hide on Overlap
  (bind _asplayer_avatar_bp (Utilities|Casting|CastToPlayerAvatar_BP OtherActor))
  (Variables|/Game/Character/PlayerAvatar_BP.PlayerAvatar_BP_C|SetisNPC? _asplayer_avatar_bp true)
  (Variables|/Game/Character/PlayerAvatar_BP.PlayerAvatar_BP_C|SetNPC%20REF _asplayer_avatar_bp self)
  (if (Variables|Companion|GetCanInteract?)
    (Utilities|FlowControl|DoOnce false
      (:Completed
        (bind _returnvalue (UserInterface|CreateWidget "/Game/Character/UI/W_Interact.W_Interact_C" 0 "Talk"))
        (bind _returnvalue_2 (AddComponent|AddWidgetComponent false))
        (bind _output_get (Variables|Default|SetInteractionWidgetComponent _returnvalue_2))
        (UserInterface|SetWidget _output_get _returnvalue)
        (Class|WidgetComponent|SetWidgetSpace _output_get "Screen")
        (Class|WidgetComponent|SetDrawatDesiredSize _output_get true)
        (Collision|SetCollisionEnabled _output_get "NoCollision")
        (Transformation|AttachComponentToComponent _output_get 0 "None" "SnapToTarget" "SnapToTarget" "SnapToTarget" true)))))

(event OnComponentEndOverlap(Sphere)
  (params (OverlappedComponent :type Primitive%20Component%20Object%20Reference) (OtherActor :type Actor%20Object%20Reference) (OtherComp :type Primitive%20Component%20Object%20Reference) (OtherBodyIndex :type Integer))
  ;[1 1 1] Interaction Text Show/Hide on Overlap
  (bind _interactionwidgetcomponent (Variables|Default|GetInteractionWidgetComponent)
    (:then
      (Components|DestroyComponent _interactionwidgetcomponent)
      (bind _asplayer_avatar_bp (Utilities|Casting|CastToPlayerAvatar_BP OtherActor))
      (Variables|/Game/Character/PlayerAvatar_BP.PlayerAvatar_BP_C|SetNPC%20REF _asplayer_avatar_bp 0)
      (Variables|/Game/Character/PlayerAvatar_BP.PlayerAvatar_BP_C|SetisNPC? _asplayer_avatar_bp false)
      (Input|EnableInput _asplayer_avatar_bp (Game|GetPlayerController 0)))
    (:else)))

(event Custom|TalkWithPlayer
  ;[1 1 1] Companion Commands
  (Animation|Montage|PlayMontage (Variables|Character|GetMesh) "/Game/Animations/animSalute1a_Montage.animSalute1a_Montage"
    (:then
      (Default|SetCompanionState (Variables|Companion|GetCompanionController) "NewEnumerator3")
      (bind _interactionwidgetcomponent (Variables|Default|GetInteractionWidgetComponent)
        (:then
          (Components|DestroyComponent _interactionwidgetcomponent))
        (:else)))))

(event Custom|Stay
  ;[1 1 1] Companion Commands
  (Default|SetCompanionState (Variables|Companion|GetCompanionController) "NewEnumerator0"))

(event Custom|Go
  (params (Location :type Vector))
  ;[1 1 1] Companion Commands
  (Default|SetGotoLocation (Variables|Companion|GetCompanionController) Location)
  (Default|SetCompanionState (Variables|Companion|GetCompanionController) "NewEnumerator0")
  (Default|SetCompanionState (Variables|Companion|GetCompanionController) "NewEnumerator2"))

(event Custom|Follow
  (params (FollowActor :type Actor%20Object%20Reference))
  ;[1 1 1] Companion Commands
  (Default|SetFollowActor (Variables|Companion|GetCompanionController) FollowActor)
  (Default|SetCompanionState (Variables|Companion|GetCompanionController) "NewEnumerator1"))

(event EventBeginPlay
  ;[1 1 1] Event Begin Play
  (bind _ascompanion_controller_bp (Utilities|Casting|CastToCompanionController_BP (AI|GetAIController self)))
  (Variables|Companion|SetCompanionController _ascompanion_controller_bp)
  (Variables|/Game/Character/AI/AI_Controller.AI_Controller_C|SetDialogueTree _ascompanion_controller_bp (Variables|Dialogue|GetDialogueTree)))

(fn ConstructionScript)

(fn GetInteractionTextAttached
  (return 0))