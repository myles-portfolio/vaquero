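; AI controller for a companion character that runs the companion behavior tree and blackboard on begin play.
; Custom events write the companion state, follow actor and go-to location into blackboard keys for the tree to read.
; Dialogue start swaps to a separate dialogue behavior tree, while dialogue end stops the brain component's logic without restarting the companion tree.
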(event Custom|SetCompanionState
  (params (State :type CompState_Enum%20Enum :default "NewEnumerator0"))
  ;[0 0 0] Set Companion State
  (AI|Components|Blackboard|SetValueasEnum (Variables|Default|GetBlackboard) (Utilities|Name|MakeLiteralName "CompanionState") State))

(event Custom|SetFollowActor
  (params (FollowActor :type Actor%20Object%20Reference))
  ;[0 0 0] Set Follow Actor
  (AI|Components|Blackboard|SetValueasObject (Variables|Default|GetBlackboard) (Utilities|Name|MakeLiteralName "FollowActor") FollowActor))

(event Custom|CompStartDialogue
  ;[0 0 0] Start Dialogue
  (AI|RunBehaviorTree (Variables|Default|GetDialogueTree)))

(event Custom|CompEndDialogue
  ;[0 0 0] End Dialogue
  (AI|Logic|StopLogic (Variables|Default|GetBrainComponent) ""))

(event Custom|SetGoToLocation
  (params (TargetLocation :type Vector))
  ;[0 0 0] Set Go To Location
  (AI|Components|Blackboard|SetValueasVector (Variables|Default|GetBlackboard) (Utilities|Name|MakeLiteralName "GoToLocation") TargetLocation))

(event EventBeginPlay
  (AI|RunBehaviorTree "/Game/Character/AI/Companion/Companion_BT.Companion_BT")
  (Class|AIController|UseBlackboard "/Game/Character/AI/Companion/Companion_BB.Companion_BB"))

(fn ConstructionScript
  (|CallParentFunction))